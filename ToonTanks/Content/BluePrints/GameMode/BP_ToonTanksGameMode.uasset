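; Game mode Blueprint for ToonTanks that shows the start and end screens of a match.
; StartGame puts the start widget on the viewport, and GameOver adds the end widget with win or loss text chosen from WonGame.
; The Escape key quits the game.
; An earlier branched version of the game-over logic remains unconnected, and BeginPlay and Tick are empty.
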(event EventBeginPlay)

(event EventTick
  (params (DeltaSeconds :type Float%20%28single-precision%29)))

(event EventStartGame
  (bind _returnvalue (UserInterface|CreateWidget "/Game/BluePrints/Widgets/WBP_StartGameWidget.WBP_StartGameWidget_C"))
  (UserInterface|Viewport|AddtoViewport _returnvalue 0))

(event EventGameOver
  (params (bWonGame :type Boolean))
  ;[1 1 1] 리팩한 로직
  (bind _returnvalue (UserInterface|CreateWidget "/Game/BluePrints/Widgets/WBP_EndGameWidget.WBP_EndGameWidget_C"))
  (UserInterface|Viewport|AddtoViewport _returnvalue 0)
  (Rendering|Components|TextRender|SetText (Variables|/Game/BluePrints/Widgets/WBP_EndGameWidget.WBP_EndGameWidget_C|GetDisplayText _returnvalue) (select bWonGame "You Won!" "You Lost! 
Click Mouse Left Button to Restart!")))

(event Input|KeyboardEvents|Escape
  (params (Key :type Key%20Structure :default "None"))
  (:Pressed
    (Game|QuitGame 0 "Quit" false)))

(fn ConstructionScript)